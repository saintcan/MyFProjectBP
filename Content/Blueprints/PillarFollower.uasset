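; PillarFollower is an actor that shuttles back and forth between the player character and a Pillar.
; It starts by targeting the player, and each Tick interpolates its location toward a point slightly above the target, without sweeping.
; Coming within a short distance sets a direction-change flag, which the next Tick consumes through a FlipFlop to switch targets.
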(event `self.ReceiveBeginPlay`
  (set `self.Target Actor` (`GameplayStatics.GetPlayerCharacter` 0)))

(event `self.ReceiveTick`
  (params (DeltaSeconds :type "Float (single-precision)"))
  (bind _returnvalue (`self.K2_GetActorLocation`))
  (bind _returnvalue_2 (`self.K2_GetActorLocation` (`self.Target Actor`)))
  (if (`self.change direction`)
    (`/Engine/EditorBlueprintResources/StandardMacros.FlipFlop`
      (:`A`
        (set `self.Target Actor` (`self.Pillar`)))
      (:`B`
        (set `self.Target Actor` (`GameplayStatics.GetPlayerCharacter` 0))))
    (set `self.change direction` false))
  (if (< (`KismetMathLibrary.Vector_Distance` _returnvalue_2 _returnvalue) 100.0)
    (set `self.change direction` true)
    (else
      (`self.K2_SetActorLocation` (`KismetMathLibrary.VInterpTo` _returnvalue (+ _returnvalue_2 (0.0 0.0 20.0)) DeltaSeconds 2.0)))))

(fn `UserConstructionScript`)