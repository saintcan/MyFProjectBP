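; Planefolw is an actor that spawns a PlayeCirclerFollower slightly above its own location when the third-person character hits it.
; It binds to its own hit event on BeginPlay and unbinds on the first hit, so a first hit from any other actor uses up the trigger and only prints a debug string.
; SpawnCirclFoll also checks and updates PlaneMap to avoid spawning twice for the same plane.
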(event `self.ReceiveBeginPlay`
  (add `self.OnActorHit` (delegate `CustomEvent_2`)))

(event `CustomEvent_2` :!signature `self.OnActorHit`
  (params (SelfActor :type "Actor Object Reference") (OtherActor :type "Actor Object Reference") (NormalImpulse :type "Vector Structure") (Hit :type "HitResult Structure (by ref)"))
  (remove `self.OnActorHit` (delegate `CustomEvent_2`))
  (`self.Spawn CirclFoll` SelfActor OtherActor))

(fn `Spawn CirclFoll`
  (params (Plane :type "Actor Object Reference") (Player :type "Actor Object Reference"))
  (locals (`Plane  Map` :type "Array of Actor Object Reference"))
  (bind _plane__map (`local.Plane  Map`))
  (if (not (`KismetArrayLibrary.Array_Contains` _plane__map Plane))
    (cast `/Game/ThirdPerson/Blueprints/BP_ThirdPersonCharacter` Player
      (:`then`
        (`|SpawnActorFromClass` "/Game/Blueprints/PlayeCirclerFollower.PlayeCirclerFollower_C" (`KismetMathLibrary.Conv_VectorToTransform` (+ (`self.K2_GetActorLocation`) (0.0 0.0 40.0))) "Undefined" "MultiplyWithRoot" null null)
        (`KismetArrayLibrary.Array_Add` _plane__map Plane))
      (:`CastFailed`
        (`KismetSystemLibrary.PrintString` "Hello")))))

(fn `UserConstructionScript`)