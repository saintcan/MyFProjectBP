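; PlayeCirclerFollower is an actor that follows the player character and circles them once it gets close.
; Each Tick, it eases toward a point slightly above the player with VInterpTo whenever it is outside a short radius.
; First entering that radius permanently sets MoveCircle, so Revolvearound then runs every frame alongside the follow.
; Revolvearound orbits the Cube component by rotating its player-relative vector around world Z, scaled by delta time.
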(event `self.ReceiveTick`
  (params (DeltaSeconds :type "Float (single-precision)"))
  (bind _returnvalue (`self.K2_GetActorLocation`))
  (bind _returnvalue_2 (`self.K2_GetActorLocation`))
  (bind _returnvalue_3 (`self.K2_GetActorLocation` (`GameplayStatics.GetPlayerCharacter` 0)))
  (bind _returnvalue_4 (`self.K2_GetActorLocation` (`GameplayStatics.GetPlayerCharacter` 0)))
  (if (`self.Move Circle`)
    (`self.Revolvearound`)
    (if (not (< (`KismetMathLibrary.Vector_Distance` _returnvalue_3 _returnvalue) 100.0))
      (`self.K2_SetActorLocation` (`KismetMathLibrary.VInterpTo` _returnvalue (+ _returnvalue_3 (0.0 0.0 20.0)) DeltaSeconds 2.0)))
    (elif (< (`KismetMathLibrary.Vector_Distance` _returnvalue_4 _returnvalue_2) 100.0)
      (set `self.Move Circle` true)
      (else
        (`self.K2_SetActorLocation` (`KismetMathLibrary.VInterpTo` _returnvalue_2 (+ _returnvalue_4 (0.0 0.0 20.0)) DeltaSeconds 2.0))))))

(fn `Revolvearound`
  (bind _output_get (set `self.Orbit Deiraction` (- (`SceneComponent.K2_GetComponentLocation` (`self.Cube`)) (`self.K2_GetActorLocation` (`GameplayStatics.GetPlayerCharacter` 0)))))
  (`SceneComponent.K2_AddWorldOffset` (`self.Cube`) (- (`KismetMathLibrary.RotateAngleAxis` _output_get (* (`GameplayStatics.GetWorldDeltaSeconds`) 90.0) (0.0 0.0 1.0)) (`self.Orbit Deiraction`)) false false))

(fn `UserConstructionScript`)