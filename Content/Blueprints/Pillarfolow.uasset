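; Pillarfolow is an actor that spawns a PillarFollower when the third-person character hits it.
; It binds its hit event on BeginPlay and unbinds it on the first hit from any actor.
; If the pillar is not yet in PlaneMap and the hitter is the character, the follower spawns just above the pillar with both references and the pillar is recorded.
; A non-character hitter only prints a debug string.
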(event `self.ReceiveBeginPlay`
  (add `self.OnActorHit` (delegate `OnActorHit_Event`)))

(event `OnActorHit_Event` :!signature `self.OnActorHit`
  (params (SelfActor :type "Actor Object Reference") (OtherActor :type "Actor Object Reference") (NormalImpulse :type "Vector Structure") (Hit :type "HitResult Structure (by ref)"))
  (remove `self.OnActorHit` (delegate `OnActorHit_Event`))
  (`self.spawn folow` SelfActor OtherActor))

(fn `spawn folow`
  (params (pillar :type "Actor Object Reference (by ref)") (player :type "Actor Object Reference"))
  (locals (`Plane  Map` :type "Array of Actor Object Reference"))
  (bind _plane__map (`local.Plane  Map`))
  (if (not (`KismetArrayLibrary.Array_Contains` _plane__map pillar))
    (bind _asbp_third_person_character (cast `/Game/ThirdPerson/Blueprints/BP_ThirdPersonCharacter` player)
      (:`then`
        (bind _returnvalue (`|SpawnActorFromClass` "/Game/Blueprints/PillarFollower.PillarFollower_C" (`KismetMathLibrary.Conv_VectorToTransform` (+ (`self.K2_GetActorLocation` pillar) (0.0 0.0 40.0))) "Undefined" "MultiplyWithRoot" null pillar null null))
        (`KismetArrayLibrary.Array_Add` _plane__map pillar)
        (set `/Game/Blueprints/PillarFollower.Player` _asbp_third_person_character _returnvalue))
      (:`CastFailed`
        (`KismetSystemLibrary.PrintString` "Hello")))))

(fn `UserConstructionScript`)