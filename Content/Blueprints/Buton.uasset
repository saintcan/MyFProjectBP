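; Buton is an interactable button that cycles its cube's material between blue, red and green.
; Overlapping its sphere shows the interact widget and sets a collision flag; ending the overlap hides and clears them.
; The Changecolor custom event advances a wrapping color index on every call, but applies the matching material only while the flag is set.
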(event `self.Sphere.OnComponentBeginOverlap`
  (params (OverlappedComponent :type "PrimitiveComponent Object Reference") (OtherActor :type "Actor Object Reference") (OtherComp :type "PrimitiveComponent Object Reference") (OtherBodyIndex :type Integer) (bFromSweep :type Boolean) (SweepResult :type "HitResult Structure (by ref)"))
  ;[1 1 1] visable interact
  (`SceneComponent.SetVisibility` (`self.interactWB`) true false)
  (set `self.CollisionCheck` true))

(event `self.Sphere.OnComponentEndOverlap`
  (params (OverlappedComponent :type "PrimitiveComponent Object Reference") (OtherActor :type "Actor Object Reference") (OtherComp :type "PrimitiveComponent Object Reference") (OtherBodyIndex :type Integer))
  ;[1 1 1] visable interact
  (`SceneComponent.SetVisibility` (`self.interactWB`) false false)
  (set `self.CollisionCheck` false))

(event `Change color`
  (bind _cube (`self.Cube`))
  ;[1 1 1] change color
  (bind _output_get (set `self.Ncolor` (+ (`self.Ncolor`) 1)))
  (if (not (<= _output_get 2))
    (set `self.Ncolor` 0))
  (if (`self.CollisionCheck`)
    (switch `int` (`self.Ncolor`)
      (:`Default`
        (`PrimitiveComponent.SetMaterial` _cube 0 "/Game/Blueprints/MaterialButon/blue.blue" :!label _label))
      (:`0`
        (goto _label))
      (:`1`
        (`PrimitiveComponent.SetMaterial` _cube 0 "/Game/Blueprints/MaterialButon/red.red"))
      (:`2`
        (`PrimitiveComponent.SetMaterial` _cube 0 "/Game/Blueprints/MaterialButon/green.green")))))

(fn `UserConstructionScript`)